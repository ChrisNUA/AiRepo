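; Throwable rock actor that makes noise where it lands, detectable through noise events.
; Interact enables physics and collision, launches the rock along the camera's forward vector with an upward boost, and sets a limited lifespan.
; The rock's component hit feeds a DoOnce gate, which reports noise, adds an audio component and spawns a steam particle effect at the impact point.
; A Reset event re-arms the gate.
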(event `/Game/Blueprints/Communication.Interact`
  (bind _rock (`self.Rock`))
  (`PrimitiveComponent.SetSimulatePhysics` _rock true)
  (`PrimitiveComponent.SetCollisionEnabled` _rock "QueryAndPhysics")
  (`PrimitiveComponent.AddImpulse` (`self.Rock`) (+ (* (`self.GetActorForwardVector` (`GameplayStatics.GetPlayerCameraManager` 0)) (`self.Impulse`)) (0.0 0.0 1000.0)) "None" false)
  (`self.SetLifeSpan` 10.0))

(event `Reset`
  (goto _label :!via `Reset`))

(event `self.Rock.OnComponentHit`
  (params (HitComponent :type "PrimitiveComponent Object Reference") (OtherActor :type "Actor Object Reference") (OtherComp :type "PrimitiveComponent Object Reference") (NormalImpulse :type "Vector Structure") (Hit :type "HitResult Structure (by ref)"))
  (bind (_bblockinghit _binitialoverlap _time _distance _location) (`GameplayStatics.BreakHitResult` Hit))
  (`/Engine/EditorBlueprintResources/StandardMacros.DoOnce` false :!label _label
    (:`Completed`
      (`AISense_Hearing.ReportNoiseEvent` _location 2.0 self 1000.0)
      (`AddComponent|NODE_AddAudioComponent-2` :`RelativeTransform` (`KismetMathLibrary.Conv_VectorToTransform` _location))
      (`GameplayStatics.SpawnEmitterAtLocation` "/Game/StarterContent/Particles/P_Steam_Lit.P_Steam_Lit" _location))))

(fn `UserConstructionScript`)